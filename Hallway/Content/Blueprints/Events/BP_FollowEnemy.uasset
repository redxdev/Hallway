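; BP_FollowEnemy is a horror gameplay event that briefly makes an enemy appear behind the player.
; It hides its mesh and registers with HorrorGameState on BeginPlay, and always reports that it can execute.
; On execution it shows the mesh, teleports behind the player pawn facing it, and plays a ghost sound there.
; It hides again after a short delay, or immediately if the teleport fails.
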(event EventExecuteEvent
  (bind _returnvalue (Game|Player|GetPlayerPawn 0))
  (bind _returnvalue_2 (Transformation|GetActorLocation _returnvalue))
  (bind _returnvalue_3 (Transformation|GetActorForwardVector _returnvalue))
  (bind _returnvalue_4 (* _returnvalue_3 -2e+02))
  (bind _returnvalue_5 (+ _returnvalue_2 _returnvalue_4))
  (Rendering|SetVisibility (Variables|Default|GetMesh) true false)
  (bind _returnvalue_6 (Transformation|Teleport _returnvalue_5 (Class|KismetMathLibrary|MakeRot 0.0 (.Yaw (Class|KismetMathLibrary|BreakRot (Math|Rotator|FindLookatRotation _returnvalue_5 _returnvalue_2))) 0.0)))
  (if _returnvalue_6
    (Audio|PlaySoundatLocation "/Game/Audio/SFX/A_Ghost01.A_Ghost01" _returnvalue_5)
    (Utilities|FlowControl|Delay 3.0))
  (Rendering|SetVisibility (Variables|Default|GetMesh) false false))

(event EventBeginPlay
  (Rendering|SetVisibility (Variables|Default|GetMesh) false false)
  (bind _ashorrorgamestate (Utilities|Casting|CastToHorrorGameState (Game|GetGameState)))
  (Class|HorrorGameState|AddGameplayEvent _ashorrorgamestate self))

(fn ConstructionScript)

(fn CanExecuteEvent
  (return true))