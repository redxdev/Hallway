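; BP_TimedObjective is an objective that completes when a HallwayCharacter stays overlapping it for a set amount of time.
; Overlap begin starts a countdown and signals the objective as started, while overlap end stops it, signals cancellation and optionally resets the remaining time.
; Tick runs the countdown, then signals completion and destroys the actor when time runs out.
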(event EventActorBeginOverlap
  (params (OtherActor :type Actor%20Object%20Reference))
  (Utilities|Casting|CastToHallwayCharacter OtherActor)
  (Variables|Objective|SetTime%20Running true)
  (Default|CallObjectiveStarted))

(event EventTick
  (params (DeltaSeconds :type Float%20%28single-precision%29))
  (if (Variables|Objective|GetTime%20Running)
    (Variables|Objective|SetTime%20Left (- (Variables|Objective|GetTime%20Left) DeltaSeconds))
    (if (<= (Variables|Objective|GetTime%20Left) 0.0)
      (Default|CallObjectiveCompleted)
      (Actor|DestroyActor))))

(event EventActorEndOverlap
  (params (OtherActor :type Actor%20Object%20Reference))
  (Utilities|Casting|CastToHallwayCharacter OtherActor)
  (Variables|Objective|SetTime%20Running false)
  (Default|CallObjectiveCanceled)
  (if (Variables|Objective|GetReset%20Time%20On%20Cancel)
    (Variables|Objective|SetTime%20Left (Variables|Objective|GetTime%20Needed))))

(event EventBeginPlay
  (Variables|Objective|SetTime%20Left (Variables|Objective|GetTime%20Needed)))

(fn ConstructionScript)