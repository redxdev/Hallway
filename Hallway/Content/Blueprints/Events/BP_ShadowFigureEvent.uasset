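; BP_ShadowFigureEvent is a horror gameplay event that makes a shadow figure flicker into view while a light flickers.
; On BeginPlay it registers itself with the HorrorGameState and hides its mesh.
; ExecuteEvent plays a timeline whose event tracks toggle the light and mesh, yawing the mesh to face the player on each mesh flicker.
; When the timeline finishes, the figure is hidden and the light is left on.
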(event EventExecuteEvent
  (bind _mesh (Variables|Default|GetMesh))
  (Timeline|Flickering%20Timeline PlayFromStart
    (:Finished
      (Rendering|SetVisibility (Variables|Default|GetMesh) false false)
      (Rendering|SetVisibility (Variables|GameplayEvent|GetLight) true false))
    (:Light%20Flicker
      (Rendering|ToggleVisibility (Variables|GameplayEvent|GetLight) false))
    (:Mesh%20Flicker
      (Rendering|ToggleVisibility _mesh false)
      (Transformation|SetWorldRotation _mesh (Class|KismetMathLibrary|MakeRot 0.0 (.Yaw (Class|KismetMathLibrary|BreakRot (Math|Rotator|FindLookatRotation (Transformation|GetWorldLocation (Variables|Default|GetMesh)) (Transformation|GetActorLocation (Game|Player|GetPlayerPawn 0))))) 0.0) false))))

(event EventBeginPlay
  (bind _ashorrorgamestate (Utilities|Casting|CastToHorrorGameState (Game|GetGameState)))
  (Class|HorrorGameState|AddGameplayEvent _ashorrorgamestate self)
  (Rendering|SetVisibility (Variables|Default|GetMesh) false false))

(fn ConstructionScript)