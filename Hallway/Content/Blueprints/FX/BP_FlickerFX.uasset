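; BP_FlickerFX is an actor that makes its Light flicker while a Character overlaps it.
; On overlap it plays the LightFlicker timeline from the start, whose event tracks toggle the light's visibility and play a flicker sound at the actor's location.
; When the timeline finishes or the Character leaves, the light is set visible again, and leaving also stops the timeline.
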(event EventActorBeginOverlap
  (params (OtherActor :type Actor%20Object%20Reference))
  (bind _light (Variables|FX|GetLight))
  (Utilities|Casting|CastToCharacter OtherActor)
  (Timeline|Light%20Flicker PlayFromStart
    (:Finished
      (Rendering|SetVisibility _light true false))
    (:Light%20Flicker
      (Rendering|ToggleVisibility _light false))
    (:Flicker%20Sound
      (Audio|PlaySoundatLocation "/Game/Audio/SFX/SC_Flicker01.SC_Flicker01" (Transformation|GetActorLocation)))))

(event EventActorEndOverlap
  (params (OtherActor :type Actor%20Object%20Reference))
  (bind _light (Variables|FX|GetLight))
  (Utilities|Casting|CastToCharacter OtherActor)
  (Rendering|SetVisibility (Variables|FX|GetLight) true false)
  (Timeline|Light%20Flicker Stop
    (:Finished
      (Rendering|SetVisibility _light true false))
    (:Light%20Flicker
      (Rendering|ToggleVisibility _light false))
    (:Flicker%20Sound
      (Audio|PlaySoundatLocation "/Game/Audio/SFX/SC_Flicker01.SC_Flicker01" (Transformation|GetActorLocation)))))

(fn ConstructionScript)