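; BP_EnemyCharacter is an enemy that halts while the player watches it and ends the game on contact.
; Each tick it runs a view-angle visibility check against the player camera, stopping movement when seen and occasionally playing a ghost sound.
; Overlapping another Character plays a scream, applies damage, prints a loss message and quits after a short delay.
; The graph contains no movement or chase logic of its own.
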(event EventActorBeginOverlap
  (params (OtherActor :type Actor%20Object%20Reference))
  (if (!= OtherActor self)
    (bind _ascharacter (Utilities|Casting|CastToCharacter OtherActor))
    (Audio|PlaySoundatLocation "/Game/Audio/SFX/A_Scream01.A_Scream01" (Transformation|GetActorLocation) 4.0)
    (Game|Damage|ApplyDamage _ascharacter 1e+02 (Pawn|GetController) self "/Engine/EngineDamageTypes/DmgTypeBP_Environmental.DmgTypeBP_Environmental_C")
    (Development|PrintString "You lose!" true true "(R=1.000000,G=0.000000,B=0.743839,A=1.000000)")
    (Utilities|FlowControl|Delay 3.0)
    (Game|QuitGame 0 "Quit")))

(event EventTick
  (params (DeltaSeconds :type Float%20%28single-precision%29))
  (bind _result (CallFunction|IsVisible self (Game|GetPlayerCameraManager 0) 45.0))
  (if _result
    (Components|Movement|StopMovementImmediately (Pawn|GetMovementComponent))
    (if (== (Math|Random|RandomInteger 1000) 0)
      (Audio|PlaySoundatLocation "/Game/Audio/SFX/A_Ghost01.A_Ghost01" (Transformation|GetActorLocation) 1.0 1.0 0.0 "/Game/Audio/SFX/Drones/Attenuation_Drone.Attenuation_Drone"))))

(fn ConstructionScript)