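; Behavior Tree task that finds the nearest TargetPoint actor lying farther than a minimum distance from the task's owner.
; On execute, it scans every TargetPoint in the world, keeping the closest one beyond MinDistance.
; It writes that actor's location to the TargetPoint Blackboard key and succeeds, or fails if it holds no valid actor.
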(event EventReceiveExecute
  (params (OwnerActor :type Actor%20Object%20Reference))
  (Variables|Default|SetClosest%20Distance 99999999999.0)
  (bind _outactors (Actor|GetAllActorsOfClass "/Script/Engine.TargetPoint"))
  (for _array_element _outactors
    (bind _returnvalue (Transformation|GetDistanceTo OwnerActor _array_element))
    (if (and (< _returnvalue (Variables|Default|GetClosest%20Distance)) (> _returnvalue (Variables|Default|GetMin%20Distance)))
      (Variables|Default|SetClosest%20Actor _array_element)
      (Variables|Default|SetClosest%20Distance _returnvalue)))
  (if (Utilities|IsValid (Variables|Default|GetClosest%20Actor))
    (AI|BehaviorTree|SetBlackboardValueasVector (Variables|Default|GetTarget%20Point) (Transformation|GetActorLocation (Variables|Default|GetClosest%20Actor)))
    (AI|BehaviorTree|FinishExecute true)
    (else
      (AI|BehaviorTree|FinishExecute false))))