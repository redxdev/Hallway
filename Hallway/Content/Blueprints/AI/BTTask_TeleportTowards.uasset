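; Behavior tree task that teleports its owner actor using the direction toward a blackboard target point.
; It scales that direction to MaxDistance, capped at the target's distance, and picks a random point within Radius around the resulting vector.
; That vector serves directly as the origin, without adding the actor's location.
; The actor lands yawed toward player 0, and the task finishes with the teleport's success result.
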(event EventReceiveExecute
  (params (OwnerActor :type Actor%20Object%20Reference))
  (bind _returnvalue (Transformation|GetActorLocation OwnerActor))
  (bind _target_point (Variables|Default|GetTarget%20Point))
  (bind _returnvalue_2 (Class|BTFunctionLibrary|GetBlackboardValueasVector _target_point))
  (bind _returnvalue_3 (- _returnvalue_2 _returnvalue))
  (bind _returnvalue_4 (Transformation|Teleport OwnerActor (Class|NavigationSystem|GetRandomPointinRadius (Math|Vector|ClampVectorSize (* (Math|Vector|Normalize _returnvalue_3) (Variables|Default|GetMax%20Distance)) 0.0 (Math|Vector|VectorLength _returnvalue_3)) (Variables|Default|GetRadius)) (Class|KismetMathLibrary|MakeRot 0.0 (.Yaw (Class|KismetMathLibrary|BreakRot (Math|Rotator|FindLookatRotation _returnvalue (Transformation|GetActorLocation (Game|GetPlayerCharacter 0))))) 0.0)))
  (AI|BehaviorTree|FinishExecute _returnvalue_4))