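; Horror scare event actor that registers with HorrorGameState and can execute when the player is within range.
; On execution, a timeline's event tracks flicker its light and the player's flashlight, play flicker audio, and toggle the initially hidden enemy mesh while turning it toward the player.
; A passed visibility check plays a scare chord and resets the timeline's time after a short delay.
; Finishing hides the mesh, restores both lights and continues the game state's event timer.
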(event EventExecuteEvent
  (bind _returnvalue (Transformation|GetActorLocation))
  (bind _ashallwaycharacter (Utilities|Casting|CastToHallwayCharacter (Game|GetPlayerCharacter 0)))
  (Timeline|Flickering%20Timeline PlayFromStart
    (:Finished
      (Rendering|SetVisibility (Variables|Default|GetMesh) false false)
      (Rendering|SetVisibility (Variables|GameplayEvent|GetLight) true false)
      (Variables|/Script/Hallway.HallwayCharacter|SetFlashlightEnabled _ashallwaycharacter true)
      (bind _ashorrorgamestate (Utilities|Casting|CastToHorrorGameState (Game|GetGameState)))
      (Class|HorrorGameState|ContinueEventTimer _ashorrorgamestate 0.7))
    (:Light%20Flicker
      (Rendering|ToggleVisibility (Variables|GameplayEvent|GetLight) false)
      (Class|HallwayCharacter|ToggleFlashlightEnabled _ashallwaycharacter))
    (:Mesh%20Flicker
      (Rendering|ToggleVisibility (Variables|Default|GetMesh) false)
      (Transformation|SetActorRotation (Class|KismetMathLibrary|MakeRot 0.0 (.Yaw (Class|KismetMathLibrary|BreakRot (Math|Rotator|FindLookatRotation (Transformation|GetActorLocation) (Transformation|GetActorLocation (Game|Player|GetPlayerPawn 0))))) 0.0))
      (bind _result (Utilities|IsVisible)
        (:Out
          (if _result
            (Development|PrintString "Visible")
            (Audio|PlaySoundatLocation "/Game/Audio/SFX/A_ScareChord01.A_ScareChord01" _returnvalue)
            (Utilities|FlowControl|Delay 0.2)
            (Timeline|Flickering%20Timeline SetNewTime)))))
    (:Flicker%20Audio
      (Audio|PlaySoundatLocation "/Game/Audio/SFX/SC_Flicker01.SC_Flicker01" _returnvalue))))

(event EventBeginPlay
  (bind _ashorrorgamestate (Utilities|Casting|CastToHorrorGameState (Game|GetGameState)))
  (Class|HorrorGameState|AddGameplayEvent _ashorrorgamestate self)
  (Rendering|SetVisibility (Variables|Default|GetMesh) false false))

(fn ConstructionScript)

(fn CanExecuteEvent
  (bind _returnvalue (Transformation|GetDistanceTo (Game|GetPlayerCharacter 0)))
  (return (<= _returnvalue 1e+03)))